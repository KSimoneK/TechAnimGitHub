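; Double door actor that swings open when a BP_ThirdPersonCharacter holding a key overlaps it.
; On overlap it casts the other actor, checks HasKey, then plays a Timeline whose DoorRotate value yaws the PortaSX and PortaDX leaves in opposite directions.
; The Open component's Play is called on every Timeline update rather than once.
; The file contains no closing logic.
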(event EventBeginPlay)

(event Collision|EventActorBeginOverlap
  (params (OtherActor :type Actor%20Object%20Reference))
  (bind _asbp_third_person_character (Utilities|Casting|CastToBP_ThirdPersonCharacter OtherActor))
  (if (Variables|/Game/ThirdPerson/Blueprints/BP_ThirdPersonCharacter.BP_ThirdPersonCharacter_C|GetHasKey _asbp_third_person_character)
    (bind _doorrotate (Timeline|Timeline Play)
      (:Update
        (Transformation|SetRelativeRotation (Variables|Default|GetPorta_SX) (Math|Rotator|MakeRotator 0.0 0.0 _doorrotate) false false)
        (Transformation|SetRelativeRotation (Variables|Default|GetPorta_DX) (Math|Rotator|MakeRotator 0.0 0.0 (* _doorrotate -1.0)) false false)
        (Audio|Components|Audio|Play (Variables|Default|Getopen) 0.0)))))

(event EventTick
  (params (DeltaSeconds :type Float%20%28single-precision%29)))

(fn ConstructionScript)