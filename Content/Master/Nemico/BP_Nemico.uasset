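; Enemy pawn Blueprint that roams the level, chases the player when it sees a pawn and plays an attack animation on reach.
; Roaming loops AIMoveTo through random reachable nearby points, pausing after each successful move.
; PawnSensing starts the chase toward player 0, while a retriggerable delay resumes roaming once sightings stop.
; CanAttack and a DoOnce gate the attack montage, resetting after its length; no damage is applied here.
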(event OnSeePawn(PawnSensing)
  (params (Pawn :type Pawn%20Object%20Reference))
  ;[0.15 0.15 0.15 0.5] Inseguimento Mostro
  (Variables|Default|SetCanAttack true)
  (Utilities|FlowControl|Sequence
    (:then_0
      (Variables|/Script/Engine.CharacterMovementComponent|SetMaxWalkSpeed (Variables|Character|GetCharacterMovement) 6e+02)
      (AI|AIMoveTo self "0, 0, 0" (Game|GetPlayerCharacter 0) 7e+01 false
        (:OnSuccess
          (if (Variables|Default|GetCanAttack)
            (Variables|Default|SetCanAttack false)
            (CallFunction|Attack)))))
    (:then_1
      (Utilities|FlowControl|RetriggerableDelay 1.0)
      (CallFunction|RoamNemico)
      (Variables|/Script/Engine.CharacterMovementComponent|SetMaxWalkSpeed (Variables|Character|GetCharacterMovement) 6e+02))))

(event Custom|RoamNemico
  ;[0.15 0.15 0.15 0.5] Roam Del Nemico
  (AI|AIMoveTo self (.RandomLocation (AI|Navigation|GetRandomReachablePointinRadius (Transformation|GetActorLocation) 1.5e+03 0 0)) 0 5.0 false
    (:OnSuccess
      (Utilities|FlowControl|Delay 2.0)
      (CallFunction|RoamNemico))))

(event Custom|Attack
  (Utilities|FlowControl|DoOnce false :!label _label
    (:Completed
      (bind _returnvalue (Animation|PlayAnimMontage "/Game/Master/Nemico/AM_Nemico.AM_Nemico" 1.0 "None"))
      (Utilities|FlowControl|Delay _returnvalue)
      (Variables|Default|SetCanAttack true)
      (goto _label Reset))))

(event EventBeginPlay
  ;[0.15 0.15 0.15 0.5] Roam Del Nemico
  (CallFunction|RoamNemico))

(event Collision|EventActorBeginOverlap
  (params (OtherActor :type Actor%20Object%20Reference)))

(fn ConstructionScript)