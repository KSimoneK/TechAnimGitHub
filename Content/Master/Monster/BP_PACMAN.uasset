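; BP_PACMAN is a monster that chases the player and ends in a jumpscare.
; Tick re-arms a looping random-delay timer each frame for AI moves to random reachable points.
; A player overlapping its box clears that timer and starts a repeating AIMoveTo chase.
; Reaching the player stops the chase, blends the view to the monster's camera, plays a bite animation with timeline-driven camera push and light, then triggers a player widget animation.
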(event OnComponentBeginOverlap(Box)
  (params (OverlappedComponent :type Primitive%20Component%20Object%20Reference) (OtherActor :type Actor%20Object%20Reference) (OtherComp :type Primitive%20Component%20Object%20Reference) (OtherBodyIndex :type Integer) (bFromSweep :type Boolean) (SweepResult :type Hit%20Result%20Structure%20%28by%20ref%29))
  (if (Actor|ActorHasTag OtherActor "Player")
    (Utilities|FlowControl|Sequence
      (:then_0
        (Utilities|Time|ClearandInvalidateTimerbyHandle (stale EventTick _returnvalue)))
      (:then_1
        (bind _returnvalue (Utilities|Time|SetTimerbyEvent (delegate Custom|CustomEvent) 0.5 true))))))

(event Custom|jumppaura
  (bind _camera (Variables|Default|GetCamera))
  (bind _relativelocation (Variables|/Script/Engine.SceneComponent|GetRelativeLocation _camera))
  (Utilities|FlowControl|Sequence
    (:then_0
      (Utilities|Time|ClearandInvalidateTimerbyHandle (stale OnComponentBeginOverlap(Box) _returnvalue)))
    (:then_1
      (bind _asbp_third_person_character (Utilities|Casting|CastToBP_ThirdPersonCharacter (Game|GetPlayerCharacter 0)))
      (Game|Player|SetViewTargetwithBlend (Game|GetPlayerController (Variables|/Script/Engine.Pawn|GetPlayerState _asbp_third_person_character)) (Components|GetOwner (Variables|Default|GetCamera)) 0.325 "VTBlend_Linear" 0.0 false)
      (Components|Animation|PlayAnimation (Variables|Character|GetMesh) "/Game/Master/Monster/Zombie_Neck_Bite.Zombie_Neck_Bite" false)
      (bind _jumppaura (Timeline|jumpaura Play)
        (:Update
          (Transformation|SetRelativeLocation _camera (Math|Vector|MakeVector (.x _relativelocation) (Math|Float|Lerp 8e+01 5e+01 _jumppaura) (.z _relativelocation)) false false)
          (Rendering|SetVisibility (Variables|Default|GetPointLight) true false))
        (:Finished
          (bind _asbp_third_person_character_2 (Utilities|Casting|CastToBP_ThirdPersonCharacter (Game|GetPlayerCharacter 0)))
          (Default|PLAYANIM (Variables|/Game/ThirdPerson/Blueprints/BP_ThirdPersonCharacter.BP_ThirdPersonCharacter_C|GetPlayer%20Widget _asbp_third_person_character_2)))))))

(event Custom|CustomEvent
  (bind _asbp_third_person_character (Utilities|Casting|CastToBP_ThirdPersonCharacter (Game|GetPlayerCharacter 0)))
  (AI|AIMoveTo self "0, 0, 0" _asbp_third_person_character 5.0 false
    (:OnSuccess
      (Utilities|FlowControl|DoOnce false
        (:Completed
          (CallFunction|Jumppaura))))))

(event Custom|RandomMovement
  (AI|AIMoveTo self (.RandomLocation (AI|Navigation|GetRandomReachablePointinRadius (Transformation|GetActorLocation) 2e+03 0 0)) 0 5.0 false))

(event EventTick
  (params (DeltaSeconds :type Float%20%28single-precision%29))
  (bind _returnvalue (Utilities|Time|SetTimerbyEvent (delegate Custom|RandomMovement) (Math|Random|RandomFloatinRange 1.0 4.0) true)))

(fn ConstructionScript)